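; TextInputManager handles player text input for a Minecraft-style game, returning either a chat line or a command result.
; ParseText formats plain text under a hardcoded nickname and sends slash-prefixed input to ParseCommand.
; ParseCommand matches the keyword against CommandKeywords and dispatches the arguments by index.
; ParseTp teleports the player using numeric block coordinates, swapping Y/Z and scaling by 100; Kill and Gamemode are empty stubs.
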(fn `ParseCommand`
  (params (CommandString :type String))
  (returns (OutText :type Text))
  (locals (Parameters :type "Array of String") (CommandIndex :type Integer))
  (bind _parameters (`local.Parameters`))
  (bind _returnvalue (`KismetStringLibrary.GetSubstring` CommandString 1 (- (`KismetStringLibrary.Len` CommandString) 1)))
  (bind _returnvalue_2 (`KismetStringLibrary.ParseIntoArray` _returnvalue))
  (if (> (`KismetStringLibrary.Len` _returnvalue) 0)
    (if (`KismetArrayLibrary.Array_IsValidIndex` _returnvalue_2)
      (for (_array_element _array_index) (`self.CommandKeywords`)
        (if (== _array_element (`|GetArrayItem` _returnvalue_2))
          (set `local.CommandIndex` _array_index)
          (break)))
      (for (_array_element_2 _array_index_2) _returnvalue_2
        (if (> _array_index_2 0)
          (`KismetArrayLibrary.Array_Add` (`local.Parameters`) _array_element_2)))
      (switch `int` (`local.CommandIndex`)
        (:`0`
          (bind _outtext (`self.ParseTp` _parameters))
          (return _outtext))
        (:`1`
          (`self.ParseKill` _parameters)
          (return "执行Kill命令"))
        (:`2`
          (`self.ParseGamemode` _parameters)
          (return "执行Gamemode命令"))))
    (else
      (return "命令为空"))))

(fn `ParseGamemode`
  (params (Parameters :type "Array of String")))

(fn `ParseKill`
  (params (InParameters :type "Array of String")))

(fn `ParseText`
  (params (InputText :type Text))
  (returns (OutText :type Text))
  (locals (InString :type String))
  (bind _returnvalue (`KismetTextLibrary.Conv_TextToString` InputText))
  (bind _instring (`local.InString`))
  (set `local.InString` _returnvalue)
  (if (`KismetStringLibrary.EqualEqual_StrStr` (`KismetStringLibrary.Left` _returnvalue 1) "/")
    (bind _outtext (`self.ParseCommand` _instring))
    (return _outtext)
    (else
      (`KismetSystemLibrary.PrintString` (`KismetStringLibrary.Concat_StrStr` "" _instring))
      (return (`|FormatText` "@{NIckName}:{Said}" "FaithBook233" (`local.InputText`))))))

(fn `ParseTp`
  (params (Parameters :type "Array of String"))
  (returns (OutText :type Text))
  (bind _parameters (`local.Parameters`))
  (bind _output (`|GetArrayItem` _parameters 2))
  (bind _output_2 (`|GetArrayItem` _parameters))
  (bind _output_3 (`|GetArrayItem` _parameters 1))
  (bind _returnvalue (`KismetStringLibrary.Conv_StringToDouble` _output))
  (bind _returnvalue_2 (`KismetStringLibrary.Conv_StringToDouble` _output_2))
  (bind _returnvalue_3 (`KismetStringLibrary.Conv_StringToDouble` _output_3))
  (if (`KismetArrayLibrary.Array_IsValidIndex` Parameters)
    (if (`KismetStringLibrary.EqualEqual_StrStr` (`KismetStringLibrary.Left` (`|GetArrayItem` Parameters) 1) "@")
      _
      (elif (== (`KismetArrayLibrary.Array_Length` Parameters) 3)
        (if (and (`KismetStringLibrary.IsNumeric` _output_2) (`KismetStringLibrary.IsNumeric` _output_3) (`KismetStringLibrary.IsNumeric` _output))
          (`self.K2_SetActorLocation` (`GameplayStatics.GetPlayerPawn` 0) (* (`KismetMathLibrary.MakeVector` _returnvalue_2 _returnvalue _returnvalue_3) 100) false false)
          (return (`|FormatText` "传送玩家到{X},{Y},{Z}" _returnvalue_2 _returnvalue_3 _returnvalue)))))))

(fn `UserConstructionScript`)