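; Voxel terrain chunk actor for a Minecraft-style world, building its block mesh on BeginPlay.
; Loads its block array from a save slot keyed by seed, chunk size and coordinate, or fills it from 2D simplex noise height layers and saves it.
; Emits only faces next to air or the chunk boundary, grouped by block ID into colliding ProceduralMesh sections with materials from a DataTable.
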(event `self.ReceiveBeginPlay`
  (`self.InitCoor`)
  (`self.ResizeBlockArray`)
  (`self.GenerateBlocks`)
  (`self.GenerateMesh`)
  (`self.UpdateMesh`))

(fn `CalcBlockID`
  (params (ZValue :type Integer) (MaxZValue :type Integer))
  (returns (BlockID :type Integer))
  (if (> ZValue MaxZValue)
    (return 1) ; 空气
    (elif (== ZValue 0)
      (return 5) ; 基岩
      (elif (and (<= ZValue MaxZValue) (> ZValue (- MaxZValue 3)))
        (return 4) ; 草方块
        (else
          (return 2) ; 石头
        )))))

(fn `CreateBlocks`
  (params (InFactor :type "Float (double-precision)" :default 0.0001))
  (locals (XOffset :type Integer) (YOffset :type Integer) (ZOffset :type Integer) (AirType :type Byte :default 1) (StoneType :type Byte :default 2))
  (bind (_returnvalue_x _returnvalue_y) (`KismetMathLibrary.BreakVector` (`self.K2_GetActorLocation`)))
  (bind _returnvalue (- (`self.ChunkSize`) 1))
  (for _index (range (+ _returnvalue 1))
    (set `local.XOffset` _index)
    (for _index_2 (range (+ _returnvalue 1))
      (set `local.YOffset` _index_2)
      (bind _returnvalue_2 (`SimplexNoiseBPLibrary.SimplexNoiseInRange2D` (+ (* (`local.XOffset`) 100.0) _returnvalue_x) (+ (* (`local.YOffset`) 100.0) _returnvalue_y) 3.0 (`KismetMathLibrary.Conv_IntToDouble` (- (`self.ChunkSize`) 1)) (`local.InFactor`)))
      (for _index_3 (range (`self.ChunkSize`))
        (bind _output_get (set `local.ZOffset` _index_3))
        (`KismetArrayLibrary.Array_Set` (`self.Blocks`) (`self.GetBlocksIndex` (`local.XOffset`) (`local.YOffset`) (`local.ZOffset`)) (`self.CalcBlockID` _output_get (`KismetMathLibrary.FFloor` _returnvalue_2)))))))

(fn `CreateFace`
  (params (FaceDirection :type "/Game/Minecraft/Blueprints/Data/Enums/Direction Enum" :default "NewEnumerator0") (InPosition :type "Vector Structure") (BlockID :type Integer))
  (locals (VerticesNum :type Integer :default 0) (TempMeshData :type "/Game/Minecraft/Blueprints/Data/Structs/MeshData Structure"))
  (bind (_tempmeshdata_vertices _tempmeshdata_triangles _tempmeshdata_uv _tempmeshdata_vertexcolors) (break `/Game/Minecraft/Blueprints/Data/Structs/MeshData` (`local.TempMeshData`)))
  (bind _tempmeshdata_vertices_2 (break `/Game/Minecraft/Blueprints/Data/Structs/MeshData` (`local.TempMeshData`)))
  (bind (_tempmeshdata_vertices_3 _tempmeshdata_triangles_2 _tempmeshdata_uv_2) (break `/Game/Minecraft/Blueprints/Data/Structs/MeshData` (`local.TempMeshData`)))
  (bind _verticesnum (`local.VerticesNum`))
  (bind (_tempmeshdata_vertices_4 _tempmeshdata_triangles_3) (break `/Game/Minecraft/Blueprints/Data/Structs/MeshData` (`local.TempMeshData`)))
  (bind (_value _returnvalue) (`BlueprintMapLibrary.Map_Find` (`self.MeshData`) BlockID))
  (bind _returnvalue_2 (`KismetMathLibrary.MakeColor` 0.0 0.0 0.0 (`KismetMathLibrary.MapRangeClamped` (`KismetMathLibrary.Conv_ByteToDouble` (`local.FaceDirection`)) 0.0 6.0 0.0 1.0)))
  (if _returnvalue
    (bind _output_get (set `local.TempMeshData` _value))
    (set `local.VerticesNum` (`KismetArrayLibrary.Array_Length` (break `/Game/Minecraft/Blueprints/Data/Structs/MeshData` _output_get))))
  (`|ExecutionSequence`
    (:`then_0`
      (`KismetArrayLibrary.Array_Append` _tempmeshdata_vertices_2 (`self.GetFaceVertices` (`local.FaceDirection`) (`local.InPosition`))))
    (:`then_1`
      (`KismetArrayLibrary.Array_Append` _tempmeshdata_triangles_3 (`|MakeArray` (+ _verticesnum 0) (+ _verticesnum 3) (+ _verticesnum 1) (+ _verticesnum 1) (+ _verticesnum 3) (+ _verticesnum 2))))
    (:`then_2`
      (`KismetArrayLibrary.Array_Append` _tempmeshdata_uv_2 (`|MakeArray` (1.0 0.0) (0.0 0.0) (0.0 1.0) (1.0 1.0) :!type "Vector2D Structure")))
    (:`then_3`
      (`KismetArrayLibrary.Array_Append` _tempmeshdata_vertexcolors (`|MakeArray` _returnvalue_2 _returnvalue_2 _returnvalue_2 _returnvalue_2)))
    (:`then_4`
      (`BlueprintMapLibrary.Map_Add` (`self.MeshData`) (`local.BlockID`) (`local.TempMeshData`)))))

(fn `GenerateBlocks`
  (bind (_coor_x _coor_y) (break `/Game/Minecraft/Blueprints/Data/Structs/Coordinate` (`self.Coor`)))
  (bind _output_get (set `self.Slot Name` (`KismetStringLibrary.Concat_StrStr` (`KismetStringLibrary.Conv_IntToString` (`self.Seed`)) "_" (`KismetStringLibrary.Conv_IntToString` (`self.ChunkSize`)) "/" (`KismetStringLibrary.Conv_IntToString` _coor_x) "," (`KismetStringLibrary.Conv_IntToString` _coor_y)))) ; 区分不同游戏，不同Chunk
  (bind _returnvalue (`GameplayStatics.DoesSaveGameExist` _output_get))
  (if _returnvalue
    (bind _returnvalue_2 (`GameplayStatics.LoadGameFromSlot` (`self.Slot Name`))) ; 加载
    (bind _aschunk_save_game (cast `/Game/Minecraft/Blueprints/Objects/ChunkSaveGame` _returnvalue_2))
    (bind _output_get_2 (set `self.ChunkSaveGameObj` _aschunk_save_game))
    (set `self.Blocks` (`/Game/Minecraft/Blueprints/Objects/ChunkSaveGame.Blocks` _output_get_2))
    (else
      (`self.CreateBlocks` 0.0001) ; 运算Blocks
      (bind _returnvalue_3 (`GameplayStatics.CreateSaveGameObject` "/Game/Minecraft/Blueprints/Objects/ChunkSaveGame.ChunkSaveGame_C"))
      (bind _output_get_3 (set `self.ChunkSaveGameObj` _returnvalue_3))
      (set `/Game/Minecraft/Blueprints/Objects/ChunkSaveGame.Blocks` (`self.Blocks`) _output_get_3)
      (bind _returnvalue_4 (`GameplayStatics.SaveGameToSlot` _output_get_3 (`self.Slot Name`))) ; 保存
    )))

(fn `GenerateMesh`
  (locals (XOffset :type Integer) (YOffset :type Integer) (ZOffset :type Integer) (CurrentDirection :type Integer))
  (for _index (range (`self.ChunkSize`))
    (set `local.XOffset` _index)
    (for _index_2 (range (`self.ChunkSize`))
      (set `local.YOffset` _index_2)
      (for _index_3 (range (`self.ChunkSize`))
        (set `local.ZOffset` _index_3)
        (if (> (`|GetArrayItem` (`self.Blocks`) (`self.GetBlocksIndex` (`local.XOffset`) (`local.YOffset`) (`local.ZOffset`))) 1)
          (for _index_4 (range 6)
            (bind _output_get (set `local.CurrentDirection` _index_4))
            (if (`self.NeedToCreateFace` (`self.GetPositionInDirection` (cast `/Game/Minecraft/Blueprints/Data/Enums/Direction` (`KismetMathLibrary.Conv_IntToByte` _output_get)) (`KismetMathLibrary.MakeVector` (`KismetMathLibrary.Conv_IntToDouble` (`local.XOffset`)) (`KismetMathLibrary.Conv_IntToDouble` (`local.YOffset`)) (`KismetMathLibrary.Conv_IntToDouble` (`local.ZOffset`)))))
              (`self.CreateFace` (cast `/Game/Minecraft/Blueprints/Data/Enums/Direction` (`KismetMathLibrary.Conv_IntToByte` _output_get)) (* (`KismetMathLibrary.MakeVector` (`KismetMathLibrary.Conv_IntToDouble` (`local.XOffset`)) (`KismetMathLibrary.Conv_IntToDouble` (`local.YOffset`)) (`KismetMathLibrary.Conv_IntToDouble` (`local.ZOffset`))) 100) (`|GetArrayItem` (`self.Blocks`) (`self.GetBlocksIndex` (`local.XOffset`) (`local.YOffset`) (`local.ZOffset`)))))))))))

(fn `GetBlockInfo`
  (params (BlockID :type Integer))
  (returns (Found :type Boolean) (`输出行` :type "/Game/Minecraft/Blueprints/Data/Structs/BlockInfo Structure"))
  (bind _returnvalue (`|GetDataTableRow` "/Game/Minecraft/Blueprints/Data/DataTable/BlockDataTable.BlockDataTable" (`KismetStringLibrary.Conv_StringToName` (`KismetStringLibrary.Conv_IntToString` BlockID)))
    (:`then`
      (return true _returnvalue))
    (:`RowNotFound`
      (return false))))

(fn `GetFaceVertices`
  (params (NewParam :type "/Game/Minecraft/Blueprints/Data/Enums/Direction Enum" :default "NewEnumerator0") (InPosition :type "Vector Structure"))
  (returns (FaceVertices1 :type "Array of Vector Structure"))
  (locals (FaceVertices :type "Array of Vector Structure"))
  (bind _returnvalue (* NewParam 4))
  (for _index (range (`KismetMathLibrary.Conv_ByteToInt` _returnvalue) (+ (`KismetMathLibrary.Conv_ByteToInt` (+ _returnvalue 3)) 1))
    (`KismetArrayLibrary.Array_Add` (`local.FaceVertices`) (+ (`|GetArrayItem` (`self.BlockVertexLocation`) (`|GetArrayItem` (`self.BlockFaceVertices`) _index)) (`local.InPosition`))))
  (return (`local.FaceVertices`)))

(fn `GetPositionInDirection`
  (params (InDirection :type "/Game/Minecraft/Blueprints/Data/Enums/Direction Enum" :default "NewEnumerator0") (InPosition :type "Vector Structure"))
  (returns (OutPosition :type "Vector Structure"))
  (return (+ InPosition (select `/Game/Minecraft/Blueprints/Data/Enums/Direction` InDirection :`NewEnumerator0` (1.0 0.0 0.0) :`NewEnumerator1` (0.0 1.0 0.0) :`NewEnumerator2` (-1.0 0.0 0.0) :`NewEnumerator3` (0.0 -1.0 0.0) :`NewEnumerator4` (0.0 0.0 1.0) :`NewEnumerator5` (0.0 0.0 -1.0) :!type "Vector Structure"))))

(fn `InitCoor`
  (bind (_returnvalue_x _returnvalue_y) (`KismetMathLibrary.BreakVector` (`self.K2_GetActorLocation`)))
  (bind _returnvalue (* (`self.ChunkSize`) 100.0))
  (set `self.Coor` (make `/Game/Minecraft/Blueprints/Data/Structs/Coordinate` (`KismetMathLibrary.FTrunc` (/ _returnvalue_x _returnvalue)) (`KismetMathLibrary.FTrunc` (/ _returnvalue_y _returnvalue)))))

(fn `NeedToCreateFace`
  (params (Position :type "Vector Structure"))
  (returns (NeedToCreateFace :type Boolean))
  (bind _x (.x Position))
  (bind _y (.y Position))
  (bind _z (.z Position))
  (bind (_position_x _position_y _position_z) (`KismetMathLibrary.BreakVector` (`local.Position`)))
  (bind _returnvalue (`KismetMathLibrary.Conv_IntToDouble` (`self.ChunkSize`)))
  (if (or (< _x 0.0) (>= _x _returnvalue) (< _y 0.0) (>= _y _returnvalue) (< _z 0.0))
    _
    (elif (>= _z (`KismetMathLibrary.Conv_IntToDouble` (`self.ChunkSize`)))
      _
      (else
        (return (== (`|GetArrayItem` (`self.Blocks`) (`self.GetBlocksIndex` (`KismetMathLibrary.FTrunc` _position_x) (`KismetMathLibrary.FTrunc` _position_y) (`KismetMathLibrary.FTrunc` _position_z))) 1)))))
  (return true))

(fn `ResizeBlockArray`
  (`KismetArrayLibrary.Array_Resize` (`self.Blocks`) (`KismetMathLibrary.FTrunc` (`KismetMathLibrary.MultiplyMultiply_FloatFloat` (`KismetMathLibrary.Conv_IntToDouble` (`self.ChunkSize`)) 3.0))))

(fn `UpdateMesh`
  (bind _meshdata (`self.MeshData`))
  (bind _proceduralmesh (`self.ProceduralMesh`))
  (bind _keys (`BlueprintMapLibrary.Map_Keys` _meshdata))
  (for _array_element _keys
    (bind _value (`BlueprintMapLibrary.Map_Find` _meshdata _array_element))
    (`ProceduralMeshComponent.CreateMeshSection_LinearColor` :`self` _proceduralmesh :`SectionIndex` _array_element :`Vertices` (break `/Game/Minecraft/Blueprints/Data/Structs/MeshData` _value) :`Triangles` (`.Triangles_15_DE7178BD42986A3902A5C9B2BE1649D8` (break `/Game/Minecraft/Blueprints/Data/Structs/MeshData` _value)) :`UV0` (`.UV_13_04F323D8420061594BFD44AF1DA02D01` (break `/Game/Minecraft/Blueprints/Data/Structs/MeshData` _value)) :`VertexColors` (`.VertexColors_14_4F73633E4E5410A3AD926EA67F5C485B` (break `/Game/Minecraft/Blueprints/Data/Structs/MeshData` _value)) :`bCreateCollision` true)
    (bind (_found `_输出行`) (`self.GetBlockInfo` _array_element))
    (if _found
      (`PrimitiveComponent.SetMaterial` _proceduralmesh _array_element (`.Material_5_D200D596459D65F54C6646A155BBC0FF` (break `/Game/Minecraft/Blueprints/Data/Structs/BlockInfo` `_输出行`))))))

(fn `UserConstructionScript`)