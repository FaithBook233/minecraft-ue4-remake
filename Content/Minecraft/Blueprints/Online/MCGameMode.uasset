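; Game mode that streams Minecraft-style world chunks around the first player's pawn.
; Each tick, UpdateLocation stores the pawn's XY in chunk units once it moves beyond a small tolerance from the last stored position.
; On change, AddChunk spawns missing grid-aligned Chunk actors within a circular RenderingRange, and RemoveChunk destroys those outside it.
; The AllChunks map, keyed by world XY, tracks spawned chunks and prevents duplicates.
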(event `self.ReceiveBeginPlay`
  (`self.UpdateLocation`)
  (`self.AddChunk`))

(event `self.ReceiveTick`
  (params (DeltaSeconds :type "Float (single-precision)"))
  (bind _hastoupdate (`self.UpdateLocation`))
  (if _hastoupdate
    (`self.AddChunk`)
    (`self.RemoveChunk`)))

(fn `AddChunk`
  (bind (_chunklocation_x _chunklocation_y) (`KismetMathLibrary.BreakVector2D` (`self.ChunkLocation`)))
  (bind _chunksize (`self.ChunkSize`))
  (bind _returnvalue (/ (`self.RenderingRange`) (`self.ChunkSize`)))
  (for _index (range (`KismetMathLibrary.FTrunc` (- _chunklocation_x _returnvalue)) (+ (`KismetMathLibrary.FTrunc` (+ _chunklocation_x _returnvalue)) 1))
    (for _index_2 (range (`KismetMathLibrary.FTrunc` (- _chunklocation_y _returnvalue)) (+ (`KismetMathLibrary.FTrunc` (+ _chunklocation_y _returnvalue)) 1))
      (bind _returnvalue_2 (`KismetMathLibrary.MakeVector2D` (* _index _chunksize) (* _index_2 _chunksize)))
      (if (and (<= (`KismetMathLibrary.Distance2D` _returnvalue_2 (* (`self.ChunkLocation`) (`self.ChunkSize`))) (`self.RenderingRange`)) (not (`.ReturnValue` (`BlueprintMapLibrary.Map_Find` (`self.AllChunks`) _returnvalue_2))))
        (bind (_x _y) (`KismetMathLibrary.BreakVector2D` _returnvalue_2))
        (bind _returnvalue_3 (`|SpawnActorFromClass` "/Game/Minecraft/Blueprints/Actors/Chunk.Chunk_C" (`KismetMathLibrary.MakeTransform` (`KismetMathLibrary.MakeVector` _x _y)) "Undefined" "OverrideRootScale" null null))
        (`BlueprintMapLibrary.Map_Add` (`self.AllChunks`) _returnvalue_2 _returnvalue_3)))))

(fn `RemoveChunk`
  (bind _allchunks (`self.AllChunks`))
  (bind _keys (`BlueprintMapLibrary.Map_Keys` (`self.AllChunks`)))
  (for _array_element _keys
    (if (> (`KismetMathLibrary.Distance2D` _array_element (* (`self.ChunkLocation`) (`self.ChunkSize`))) (`self.RenderingRange`))
      (bind (_value _returnvalue) (`BlueprintMapLibrary.Map_Find` _allchunks _array_element))
      (if _returnvalue
        (`self.K2_DestroyActor` _value)
        (`BlueprintMapLibrary.Map_Remove` _allchunks _array_element)))))

(fn `UpdateLocation`
  (returns (HasToUpdate :type Boolean))
  (bind (_returnvalue_x _returnvalue_y) (`KismetMathLibrary.BreakVector` (`self.K2_GetActorLocation` (`GameplayStatics.GetPlayerPawn` 0))))
  (bind _returnvalue (`KismetMathLibrary.MakeVector2D` _returnvalue_x _returnvalue_y))
  (if (== _returnvalue (* (`self.ChunkLocation`) (`self.ChunkSize`)) :`ErrorTolerance` 100.0)
    (return false)
    (else
      (set `self.ChunkLocation` (/ _returnvalue (`self.ChunkSize`)))
      (return true))))

(fn `UserConstructionScript`)