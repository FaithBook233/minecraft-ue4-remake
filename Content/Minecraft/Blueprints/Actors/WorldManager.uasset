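; World manager actor for a Minecraft-style voxel world that generates seeded terrain chunks around the player.
; A looping timer tracks the player's chunk coordinate, creates missing chunks within render range and runs the terrain generator on them.
; Queued blocks become instances on per-block-type instanced mesh components, built from a data table at construction, with GlobalInfo holding shared state.
; Chunk removal is disconnected, so loaded chunks persist.
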(event `self.ReceiveBeginPlay`
  (`SimplexNoiseBPLibrary.setNoiseSeed` (`self.Seed`))
  (bind _returnvalue (`KismetSystemLibrary.K2_SetTimerDelegate` (delegate `Update`) (`self.UpdateDeltaTime`) true))
  (set `self.Up[dateTImer` _returnvalue))

(event `Update`
  (`self.UpdateLocation`)
  (`self.AddChunk`)
  (`self.UpdateMesh`))

(event `self.ReceiveTick`
  (params (DeltaSeconds :type "Float (single-precision)")))

(fn `AddChunk`
  (locals (NewChunkPosition :type "Vector2D Structure"))
  (bind _renderingrange (`self.RenderingRange`))
  (bind (_lastplayercoor_x _lastplayercoor_y) (`KismetMathLibrary.BreakVector2D` (`self.LastPlayerCoor`)))
  (bind _returnvalue (`KismetMathLibrary.FFloor` _lastplayercoor_y))
  (bind _returnvalue_2 (`KismetMathLibrary.FFloor` _lastplayercoor_x))
  (for _index (range (- _returnvalue_2 _renderingrange) (+ (+ _returnvalue_2 _renderingrange) 1))
    (for _index_2 (range (- _returnvalue _renderingrange) (+ (+ _returnvalue _renderingrange) 1))
      (bind _output_get (set `local.NewChunkPosition` (`KismetMathLibrary.MakeVector2D` (`KismetMathLibrary.Conv_IntToDouble` _index) (`KismetMathLibrary.Conv_IntToDouble` _index_2))))
      (if (not (`BlueprintMapLibrary.Map_Contains` (`/Game/Minecraft/Blueprints/Components/GlobalInfo.ChunksLoaded` (`self.GlobalInfo`)) _output_get))
        (bind _returnvalue_3 (`|AddComponentByClass` "/Game/Minecraft/Blueprints/Components/Chunk.Chunk_C" (`local.NewChunkPosition`)))
        (`BlueprintMapLibrary.Map_Add` (`/Game/Minecraft/Blueprints/Components/GlobalInfo.ChunksLoaded` (`self.GlobalInfo`)) (`local.NewChunkPosition`) _returnvalue_3)
        (`/Game/Minecraft/Blueprints/Components/TerrainGeneratorBase.Generate Terrain` (`self.TerrainGeneratorBase`) (`self.GlobalInfo`) _returnvalue_3)))))

(fn `DrawDebugShapes`
  (bind _keys (`BlueprintMapLibrary.Map_Keys` (`/Game/Minecraft/Blueprints/Components/GlobalInfo.ChunksLoaded` (`self.GlobalInfo`))))
  (for _array_element _keys
    (`KismetSystemLibrary.DrawDebugSphere` (`self.ChunkPositionToLocation` _array_element))))

(fn `InitGlobalInfo`
  (bind _globalinfo (`self.GlobalInfo`))
  (set `/Game/Minecraft/Blueprints/Components/GlobalInfo.ChunkHeight` (`self.ChunkHeight`) _globalinfo)
  (set `/Game/Minecraft/Blueprints/Components/GlobalInfo.ChunkWidth` (`self.ChunkWidth`) _globalinfo))

(fn `InitIntancedMeshComp`
  (locals (NewInstancedMeshComp :type "InstancedStaticMeshComponent Object Reference") (CurrentIndex :type Integer))
  (bind _outrownames (`DataTableFunctionLibrary.GetDataTableRowNames` "/Game/Minecraft/Blueprints/Data/DataTable/BlockDataTable.BlockDataTable"))
  (for _index (range 2 (`KismetArrayLibrary.Array_Length` _outrownames))
    (set `local.CurrentIndex` _index)
    (bind _returnvalue (`AddComponent|NODE_AddInstancedStaticMeshComponent-0`))
    (bind _output_get (set `local.NewInstancedMeshComp` _returnvalue))
    (bind _returnvalue_2 (`StaticMeshComponent.SetStaticMesh` _output_get "/Game/Minecraft/Meshes/Block.Block"))
    (if _returnvalue_2
      (bind _returnvalue_3 (`|GetDataTableRow` "/Game/Minecraft/Blueprints/Data/DataTable/BlockDataTable.BlockDataTable" (`KismetStringLibrary.Conv_StringToName` (`KismetStringLibrary.Conv_IntToString` (`local.CurrentIndex`))))
        (:`then`
          (`PrimitiveComponent.SetMaterial` (`local.NewInstancedMeshComp`) 0 (`.Material_5_D200D596459D65F54C6646A155BBC0FF` (break `/Game/Minecraft/Blueprints/Data/Structs/BlockInfo` _returnvalue_3)))
          (`BlueprintMapLibrary.Map_Add` (`self.InstancedMesnComp`) (`local.CurrentIndex`) (`local.NewInstancedMeshComp`)))))))

(fn `RemoveChunk`
  (locals (CurrentCoor :type "Vector2D Structure")))

(fn `UpdateLocation`
  (bind (_lastplayercoor_x _lastplayercoor_y) (`KismetMathLibrary.BreakVector2D` (`self.LastPlayerCoor`)))
  (bind (_returnvalue_x _returnvalue_y) (`KismetMathLibrary.BreakVector` (`self.K2_GetActorLocation` (`GameplayStatics.GetPlayerPawn` 0))))
  (bind _returnvalue (`KismetMathLibrary.MakeVector2D` _returnvalue_x _returnvalue_y))
  (bind (_returnvalue_x_2 _returnvalue_y_2) (`KismetMathLibrary.BreakVector2D` (/ _returnvalue (`self.GetChunkWidth`))))
  (if (or (> (`KismetMathLibrary.Abs` (- _returnvalue_x_2 _lastplayercoor_x)) 1.0) (> (`KismetMathLibrary.Abs` (- _returnvalue_y_2 _lastplayercoor_y)) 1.0))
    (set `self.LastPlayerCoor` (/ _returnvalue (`self.GetChunkWidth`)))))

(fn `UpdateMesh`
  (bind _globalinfo (`self.GlobalInfo`))
  (bind _blockstodisplay (`/Game/Minecraft/Blueprints/Components/GlobalInfo.BlocksToDisplay` _globalinfo))
  (bind _keys (`BlueprintMapLibrary.Map_Keys` _blockstodisplay))
  (for _array_element _keys
    (bind (_value _returnvalue) (`BlueprintMapLibrary.Map_Find` (`self.InstancedMesnComp`) (`BlueprintMapLibrary.Map_Find` _blockstodisplay _array_element)))
    (if _returnvalue
      (`InstancedStaticMeshComponent.AddInstance` _value (`KismetMathLibrary.MakeTransform` _array_element))
      (`BlueprintMapLibrary.Map_Add` (`/Game/Minecraft/Blueprints/Components/GlobalInfo.BlocksDisplayed` _globalinfo) _array_element)))
  (`BlueprintMapLibrary.Map_Clear` _blockstodisplay))

(fn `UserConstructionScript`
  (`self.InitIntancedMeshComp`)
  (`self.InitGlobalInfo`))