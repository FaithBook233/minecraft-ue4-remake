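; MCPlayerController is the player controller for a Minecraft-style game, managing the player's HUD and UI input.
; On BeginPlay it creates the MainUI widget and adds it to the viewport.
; Chat and Command input actions call MainUI to start text or command entry.
; ShowDebugInfo toggles a DebugInfo overlay by creating it above the HUD or removing and clearing it.
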(event `InputAction|ShowDebugInfo`
  (params (Key :type "Key Structure"))
  (bind _debuginfoui (`self.DebugInfoUI`))
  (:`Pressed`
    (`/Engine/EditorBlueprintResources/StandardMacros.IsValid` _debuginfoui
      (:`Is Valid`
        (`Widget.RemoveFromParent` _debuginfoui)
        (set `self.DebugInfoUI` null) ; nullptr
      )
      (:`Is Not Valid`
        (bind _returnvalue (`|CreateWidget` "/Game/Minecraft/Blueprints/UI/DebugInfo.DebugInfo_C" self))
        (bind _output_get (set `self.DebugInfoUI` _returnvalue))
        (`UserWidget.AddToViewport` _output_get 10)))))

(event `self.ReceiveBeginPlay`
  (bind _returnvalue (`|CreateWidget` "/Game/Minecraft/Blueprints/UI/MainUI.MainUI_C" self))
  (bind _output_get (set `self.MainUI` _returnvalue))
  (`UserWidget.AddToViewport` _output_get 0))

(event `InputAction|Chat`
  (params (Key :type "Key Structure"))
  (:`Pressed`
    (`/Game/Minecraft/Blueprints/UI/MainUI.StartInputText` (`self.MainUI`))))

(event `InputAction|Command`
  (params (Key :type "Key Structure"))
  (:`Pressed`
    (`/Game/Minecraft/Blueprints/UI/MainUI.StartInputCommand` (`self.MainUI`))))

(fn `UserConstructionScript`)