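; Minecraft-style voxel chunk actor that builds its own block terrain as a procedural mesh on BeginPlay.
; CreateBlocks fills a flattened 3D block array with stone or air, using 2D simplex noise at world position as the column height.
; GenerateMesh culls hidden faces, adding quads only where solid blocks border air or the chunk edge.
; UpdateMesh uploads the vertices, triangles and UVs as one shadowless mesh section.
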(event `self.ReceiveBeginPlay`
  (`PrimitiveComponent.SetCastShadow` (`self.ProceduralMesh`) false)
  (`self.ResizeBlockArray`)
  (`self.CreateBlocks` 0.0001)
  (`self.GenerateMesh`)
  (`self.UpdateMesh`))

(fn `CreateBlocks`
  (params (InFactor :type "Float (double-precision)" :default 0.0001))
  (locals (XOffset :type Integer) (YOffset :type Integer) (ZOffset :type Integer) (AirType :type "/Game/Minecraft/Blueprints/Data/Enums/BlockType Enum" :default "NewEnumerator1") (StoneType :type "/Game/Minecraft/Blueprints/Data/Enums/BlockType Enum" :default "NewEnumerator2"))
  (bind (_returnvalue_x _returnvalue_y) (`KismetMathLibrary.BreakVector` (`self.K2_GetActorLocation`)))
  (bind _returnvalue (- (`self.ChunkSize`) 1))
  (for _index (range (+ _returnvalue 1))
    (set `local.XOffset` _index)
    (for _index_2 (range (+ _returnvalue 1))
      (set `local.YOffset` _index_2)
      (bind _returnvalue_2 (`SimplexNoiseBPLibrary.SimplexNoiseInRange2D` (+ (`self.GetLocationFromIndex` (`local.XOffset`)) _returnvalue_x) (+ (`self.GetLocationFromIndex` (`local.YOffset`)) _returnvalue_y) 0.0 (`KismetMathLibrary.Conv_IntToDouble` (/ (`self.ChunkSize`) 2)) (`local.InFactor`)))
      (for _index_3 (range (`self.ChunkSize`))
        (set `local.ZOffset` _index_3)
        (`KismetArrayLibrary.Array_Set` (`self.Blocks`) (`self.GetBlocksIndex` (`local.XOffset`) (`local.YOffset`) (`local.ZOffset`)) (select `bool` (<= _index_3 (`KismetMathLibrary.FFloor` _returnvalue_2)) :`false` (`local.AirType`) :`true` (`local.StoneType`)))))))

(fn `CreateFace`
  (params (FaceDirection :type "/Game/Minecraft/Blueprints/Data/Enums/Direction Enum" :default "NewEnumerator0") (InPosition :type "Vector Structure"))
  (locals (VerticesNum :type Integer :default 0))
  (bind _verticesnum (`local.VerticesNum`))
  (set `local.VerticesNum` (`KismetArrayLibrary.Array_Length` (`self.Vertices`)))
  (`|ExecutionSequence`
    (:`then_0`
      (`KismetArrayLibrary.Array_Append` (`self.Vertices`) (`self.GetFaceVertices` FaceDirection InPosition)))
    (:`then_1`
      (`KismetArrayLibrary.Array_Append` (`self.Triangles`) (`|MakeArray` (+ _verticesnum 0) (+ _verticesnum 3) (+ _verticesnum 1) (+ _verticesnum 1) (+ _verticesnum 3) (+ _verticesnum 2))))
    (:`then_2`
      (`KismetArrayLibrary.Array_Append` (`self.UV0`) (`|MakeArray` (1.0 1.0) (1.0 0.0) (0.0 0.0) (0.0 1.0) :!type "Vector2D Structure")))))

(fn `GenerateMesh`
  (locals (XOffset :type Integer) (YOffset :type Integer) (ZOffset :type Integer) (CurrentDirection :type Integer))
  (for _index (range (`self.ChunkSize`))
    (set `local.XOffset` _index)
    (for _index_2 (range (`self.ChunkSize`))
      (set `local.YOffset` _index_2)
      (for _index_3 (range (`self.ChunkSize`))
        (set `local.ZOffset` _index_3)
        (if (> (`|GetArrayItem` (`self.Blocks`) (`self.GetBlocksIndex` (`local.XOffset`) (`local.YOffset`) (`local.ZOffset`))) 1)
          (for _index_4 (range 6)
            (bind _output_get (set `local.CurrentDirection` _index_4))
            (if (`self.NeedToCreateFace` (`self.GetPositionInDirection` (cast `/Game/Minecraft/Blueprints/Data/Enums/Direction` (`KismetMathLibrary.Conv_IntToByte` _output_get)) (`KismetMathLibrary.MakeVector` (`KismetMathLibrary.Conv_IntToDouble` (`local.XOffset`)) (`KismetMathLibrary.Conv_IntToDouble` (`local.YOffset`)) (`KismetMathLibrary.Conv_IntToDouble` (`local.ZOffset`)))))
              (`self.CreateFace` (cast `/Game/Minecraft/Blueprints/Data/Enums/Direction` (`KismetMathLibrary.Conv_IntToByte` _output_get)) (* (`KismetMathLibrary.MakeVector` (`KismetMathLibrary.Conv_IntToDouble` (`local.XOffset`)) (`KismetMathLibrary.Conv_IntToDouble` (`local.YOffset`)) (`KismetMathLibrary.Conv_IntToDouble` (`local.ZOffset`))) 100)))))))))

(fn `GetFaceVertices`
  (params (NewParam :type "/Game/Minecraft/Blueprints/Data/Enums/Direction Enum" :default "NewEnumerator0") (InPosition :type "Vector Structure"))
  (returns (FaceVertices1 :type "Array of Vector Structure"))
  (locals (FaceVertices :type "Array of Vector Structure"))
  (bind _returnvalue (* NewParam 4))
  (for _index (range (`KismetMathLibrary.Conv_ByteToInt` _returnvalue) (+ (`KismetMathLibrary.Conv_ByteToInt` (+ _returnvalue 3)) 1))
    (`KismetArrayLibrary.Array_Add` (`local.FaceVertices`) (+ (`|GetArrayItem` (`self.BlockVertexLocation`) (`|GetArrayItem` (`self.BlockFaceVertices`) _index)) (`local.InPosition`))))
  (return (`local.FaceVertices`)))

(fn `GetPositionInDirection`
  (params (InDirection :type "/Game/Minecraft/Blueprints/Data/Enums/Direction Enum" :default "NewEnumerator0") (InPosition :type "Vector Structure"))
  (returns (OutPosition :type "Vector Structure"))
  (return (+ InPosition (select `/Game/Minecraft/Blueprints/Data/Enums/Direction` InDirection :`NewEnumerator0` (1.0 0.0 0.0) :`NewEnumerator1` (0.0 1.0 0.0) :`NewEnumerator2` (-1.0 0.0 0.0) :`NewEnumerator3` (0.0 -1.0 0.0) :`NewEnumerator4` (0.0 0.0 1.0) :`NewEnumerator5` (0.0 0.0 -1.0) :!type "Vector Structure"))))

(fn `NeedToCreateFace`
  (params (Position :type "Vector Structure"))
  (returns (NeedToCreateFace :type Boolean))
  (bind _x (.x Position))
  (bind _y (.y Position))
  (bind _z (.z Position))
  (bind (_position_x _position_y _position_z) (`KismetMathLibrary.BreakVector` (`local.Position`)))
  (bind _returnvalue (`KismetMathLibrary.Conv_IntToDouble` (`self.ChunkSize`)))
  (if (or (< _x 0.0) (>= _x _returnvalue) (< _y 0.0) (>= _y _returnvalue) (< _z 0.0))
    _
    (elif (>= _z (`KismetMathLibrary.Conv_IntToDouble` (`self.ChunkSize`)))
      _
      (else
        (return (== (`|GetArrayItem` (`self.Blocks`) (`self.GetBlocksIndex` (`KismetMathLibrary.FTrunc` _position_x) (`KismetMathLibrary.FTrunc` _position_y) (`KismetMathLibrary.FTrunc` _position_z))) 1)))))
  (return true))

(fn `ResizeBlockArray`
  (`KismetArrayLibrary.Array_Resize` (`self.Blocks`) (`KismetMathLibrary.FTrunc` (`KismetMathLibrary.MultiplyMultiply_FloatFloat` (`KismetMathLibrary.Conv_IntToDouble` (`self.ChunkSize`)) 3.0))))

(fn `UpdateMesh`
  (`ProceduralMeshComponent.CreateMeshSection_LinearColor` :`self` (`self.ProceduralMesh`) :`Vertices` (`self.Vertices`) :`Triangles` (`self.Triangles`) :`UV0` (`self.UV0`)))

(fn `UserConstructionScript`)