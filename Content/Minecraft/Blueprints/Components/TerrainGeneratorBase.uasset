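; Base terrain generator component for a Minecraft-style voxel world that creates the surface blocks of a given chunk.
; GenerateTerrain loops over the chunk's square grid, offsets each column into world space and derives its height from 2D simplex noise snapped to whole blocks.
; It writes one block per column, with a hardcoded debug ID, into GlobalInfo's block ID and display maps, leaving the space beneath unfilled.
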(fn `Generate Terrain`
  (params (GlobalInfo :type "/Game/Minecraft/Blueprints/Components/GlobalInfo Object Reference") (Chunk :type "/Game/Minecraft/Blueprints/Components/Chunk Object Reference"))
  (locals (NewBlockVector2D :type "Vector2D Structure"))
  (bind _chunkwidth (`/Game/Minecraft/Blueprints/Components/GlobalInfo.ChunkWidth` GlobalInfo))
  (bind (_newblockvector2d_x _newblockvector2d_y) (`KismetMathLibrary.BreakVector2D` (`local.NewBlockVector2D`)))
  (bind _returnvalue (- _chunkwidth 1))
  (for _index (range (+ _returnvalue 1))
    (for _index_2 (range (+ _returnvalue 1))
      (bind _output_get (set `local.NewBlockVector2D` (+ (`KismetMathLibrary.MakeVector2D` (`KismetMathLibrary.Conv_IntToDouble` (* _index_2 100)) (`KismetMathLibrary.Conv_IntToDouble` (* _index 100))) (* (`/Game/Minecraft/Blueprints/Components/Chunk.ChunkPosition` Chunk) (* _chunkwidth 100.0)))))
      (bind _returnvalue_2 (`SimplexNoiseBPLibrary.SimplexNoiseInRange2D` (`KismetMathLibrary.BreakVector2D` _output_get) (`.Y` (`KismetMathLibrary.BreakVector2D` _output_get)) 3.0 32.0 0.0001))
      (bind _returnvalue_3 (* (`KismetMathLibrary.FTrunc` _returnvalue_2) 100.0))
      ;[1 1 1] Debug 4
      (`BlueprintMapLibrary.Map_Add` (`/Game/Minecraft/Blueprints/Components/GlobalInfo.GlobalBlocksID` GlobalInfo) (`KismetMathLibrary.MakeVector` _newblockvector2d_x _newblockvector2d_y _returnvalue_3) 4)
      (`BlueprintMapLibrary.Map_Add` (`/Game/Minecraft/Blueprints/Components/GlobalInfo.BlocksToDisplay` GlobalInfo) (`KismetMathLibrary.MakeVector` _newblockvector2d_x _newblockvector2d_y _returnvalue_3) 4))))